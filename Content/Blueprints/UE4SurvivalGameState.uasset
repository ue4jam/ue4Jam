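; Survival game state Blueprint that keeps a shared registry of the level's light source actors.
; On BeginPlay it fills the registry with every actor tagged "LightSource".
; Accessor functions return the list, add an actor to it and remove an entry by index.
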(event `self.ReceiveBeginPlay`
  (bind _outactors (`GameplayStatics.GetAllActorsWithTag` "LightSource"))
  (set `self.LightSourceRefs` _outactors))

(fn `AddLightSource`
  (params (LightSource :type "Actor Object Reference"))
  (returns (Index :type Integer))
  (bind _returnvalue (`KismetArrayLibrary.Array_Add` (`self.LightSourceRefs`) LightSource))
  (return _returnvalue))

(fn `GetLightSources`
  (returns (LightSourceRefs :type "Array of Actor Object Reference"))
  (return (`self.LightSourceRefs`)))

(fn `RemoveLightSource`
  (params (Index :type Integer))
  (`KismetArrayLibrary.Array_Remove` (`self.LightSourceRefs`) Index)
  (return))

(fn `UserConstructionScript`)