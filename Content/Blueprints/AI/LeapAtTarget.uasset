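; Behavior tree task that makes an EnemyCharacterBP enemy leap along its facing direction.
; On execute it sets IsLeaping, launches the character forward with a strong impulse and plays the Skull01 sound at its location.
; After a short fixed delay it clears the flag and finishes successfully, without checking for landing or reading a target.
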(event `self.ReceiveExecuteAI`
  (params (OwnerController :type "AIController Object Reference") (ControlledPawn :type "Pawn Object Reference"))
  (bind _asenemy_character_bp (cast `/Game/Blueprints/Characters/EnemyCharacterBP` ControlledPawn))
  (set `/Game/Blueprints/Characters/EnemyCharacterBP.IsLeaping` true _asenemy_character_bp)
  (`Character.LaunchCharacter` _asenemy_character_bp (* (`KismetMathLibrary.Conv_RotatorToVector` (`Actor.K2_GetActorRotation` _asenemy_character_bp)) 5000.0) false false)
  (`GameplayStatics.PlaySoundAtLocation` "/Game/Audio/Skull01.Skull01" (`Actor.K2_GetActorLocation` _asenemy_character_bp))
  (`KismetSystemLibrary.Delay` 0.2)
  (set `/Game/Blueprints/Characters/EnemyCharacterBP.IsLeaping` false _asenemy_character_bp)
  (`self.FinishExecute` true))