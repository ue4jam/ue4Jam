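; EnemyAI is an AI controller for enemies that runs the BT_EnemyBasic behavior tree on BeginPlay.
; On perception updates, it writes the first perceived actor that implements IDamageable and has the "Friendly" tag to a blackboard object key.
; A TrackPlayer event moves the AI toward the player character, but the looping timer that would call it is disconnected.
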(event `self.ReceiveBeginPlay`
  (`self.RunBehaviorTree` "/Game/Blueprints/AI/BT_EnemyBasic.BT_EnemyBasic"))

(event `TrackPlayer`
  (`AITask_MoveTo.AIMoveTo` self (0.0 0.0 0.0) (`GameplayStatics.GetPlayerCharacter` 0)))

(event `self.AIPerception.OnPerceptionUpdated`
  (params (UpdatedActors :type "Array of Actor Object Reference"))
  (for _array_element UpdatedActors
    (if (`KismetSystemLibrary.DoesImplementInterface` _array_element "/Game/Blueprints/Interfaces/iDamageable.iDamageable_C")
      (if (`self.ActorHasTag` _array_element "Friendly")
        (`BlackboardComponent.SetValueAsObject` (`AIBlueprintHelperLibrary.GetBlackboard` null) (`self.ActorKeyName`) _array_element)
        (break)))))

(fn `UserConstructionScript`)