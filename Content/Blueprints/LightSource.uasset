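; LightSource is an actor that registers itself as a light source with the survival game state and has a limited lifespan.
; Its construction script applies the LifeSpan variable, casts the game state to UE4SurvivalGameState, calls AddLightSource on it and stores the returned IndexNumber.
; The event graph does nothing: its events are empty, and nodes for a looping timer that checks for life ending are left unconnected.
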(event `self.ReceiveBeginPlay`)

(event `self.ReceiveTick`
  (params (DeltaSeconds :type "Float (single-precision)")))

(event `CheckIfLifeEnding`)

(fn `UserConstructionScript`
  (`self.SetLifeSpan` (`self.LifeSpan`))
  (bind _asue4survival_game_state (cast `/Game/Blueprints/UE4SurvivalGameState` (`GameplayStatics.GetGameState`)))
  (set `self.GameStateRef` _asue4survival_game_state)
  (bind _index (`/Game/Blueprints/UE4SurvivalGameState.AddLightSource` (`self.GameStateRef`) self))
  (set `self.IndexNumber` _index))