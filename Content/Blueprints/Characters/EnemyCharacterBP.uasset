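; Enemy character Blueprint that is hurt by light, attacks the player on overlap and drops light energy when killed.
; A one-second timer asks the game state whether it is lit and applies light damage through AffectHealth.
; Overlapping the player starts a repeating damage timer, with an immediate once-per-contact hit when leaping, cleared when overlap ends.
; On death it disables movement, spawns LightEnergyDroplets at random nearby reachable points and destroys itself.
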(event `self.ReceiveBeginPlay`
  ;[1 1 1] Begin Play
  (`parent.ReceiveBeginPlay`)
  (`|ExecutionSequence`
    (:`then_0`
      (bind _asue4survival_game_state (cast `/Game/Blueprints/States/UE4SurvivalGameState` (`GameplayStatics.GetGameState`)))
      (set `self.GameStateRef` _asue4survival_game_state))
    (:`then_1`
      (`KismetSystemLibrary.K2_SetTimer` null "DamageIfInLight" 1.0 true))))

(event `DamageIfInLight`
  ;[1 1 1] Damage If In Light
  (bind _isinlight (`/Game/Blueprints/States/UE4SurvivalGameState.CheckIfInLight` (`self.GameStateRef`) self))
  (if _isinlight
    (`self.AffectHealth` (`self.DamageFromLight`))))

(event `self.AffectHealth`
  (params (Delta :type "Float (single-precision)"))
  ;[1 1 1] Affect Health
  (`self.CalculateHealth` Delta)
  (if (`self.isDead`)
    (`CharacterMovementComponent.DisableMovement` (`self.CharacterMovement`))
    (`self.SpawnDroplets`)
    (`self.K2_DestroyActor`)))

(event `self.ReceiveActorBeginOverlap`
  (params (OtherActor :type "Actor Object Reference"))
  (bind _asplayer_character_bp (cast `/Game/Blueprints/Characters/PlayerCharacterBP` OtherActor))
  (set `self.PlayerRef` _asplayer_character_bp)
  (if (`self.IsLeaping`)
    (`/Engine/EditorBlueprintResources/StandardMacros.DoOnce` false :!label _label
      (:`Completed`
        (`self.DamagePlayer`))))
  (`KismetSystemLibrary.K2_SetTimer` null "DamagePlayer" (/ 1.0 (`self.AttacksPerSecond`)) true))

(event `self.ReceiveActorEndOverlap`
  (params (OtherActor :type "Actor Object Reference"))
  (if (== OtherActor (`self.PlayerRef`))
    (`KismetSystemLibrary.K2_ClearTimer` null "DamagePlayer")
    (goto _label :!via `Reset`)))

(event `DamagePlayer`
  (`/Game/Blueprints/Characters/PlayerCharacterBP.AffectHealth` (`self.PlayerRef`) (`self.Damage`)))

(fn `GetRandomPointInSpawnVolume`
  (returns (Location :type "Vector Structure"))
  (return (`NavigationSystem.K2_GetRandomReachablePointInRadius` (+ (`self.K2_GetActorLocation` self) (`KismetMathLibrary.RandomFloatInRange` -10.0 10.0)) 100.0)))

(fn `SpawnDroplets`
  (locals (Count :type Integer))
  (bind _output_get (set `local.Count` 0))
  (while (< _output_get (`self.DropletCount`))
    (`|SpawnActorFromClass` "/Game/Blueprints/Actors/LightEnergyDroplet.LightEnergyDroplet_C" (`KismetMathLibrary.MakeTransform` (`self.GetRandomPointInSpawnVolume`)) "AdjustIfPossibleButAlwaysSpawn" "OverrideRootScale" null null)
    (`/Engine/EditorBlueprintResources/StandardMacros.IncrementInt` (`local.Count`)))
  (return))

(fn `UserConstructionScript`
  (`parent.UserConstructionScript`))