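; BaseCharacterBP is a base character Blueprint that tracks health and death state.
; CalculateHealth adds a signed delta to Health, then calls CalculateIsDead, which sets IsDead when Health is at or below zero and clears it otherwise.
; Health is not clamped, and the event graph and construction script contain no logic.
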(fn `CalculateHealth`
  (params (Delta :type "Float (double-precision)"))
  (set `self.Health` (+ (`self.Health`) Delta))
  (`self.CalculateIsDead`)
  (return))

(fn `CalculateIsDead`
  (if (<= (`self.Health`) 0.0)
    (set `self.isDead` true)
    (else
      (set `self.isDead` false)))
  (return))

(fn `UserConstructionScript`)