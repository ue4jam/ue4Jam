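; Enemy character Blueprint for a survival game in which light hurts enemies.
; On BeginPlay it caches the UE4SurvivalGameState and starts a looping one-second timer that asks the game state whether the enemy is in light.
; When lit, it applies its light damage to health, destroying itself if that leaves it dead, and prints its health each tick of the timer as debug output.
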(event `self.ReceiveBeginPlay`
  ;[1 1 1] Begin Play
  (`parent.ReceiveBeginPlay`)
  (`|ExecutionSequence`
    (:`then_0`
      (bind _asue4survival_game_state (cast `/Game/Blueprints/UE4SurvivalGameState` (`GameplayStatics.GetGameState`)))
      (set `self.GameStateRef` _asue4survival_game_state))
    (:`then_1`
      (`KismetSystemLibrary.K2_SetTimer` null "DamageIfInLight" 1.0 true))))

(event `DamageIfInLight`
  ;[1 1 1] Damage If In Light
  (bind _isinlight (`/Game/Blueprints/UE4SurvivalGameState.CheckIfInLight` (`self.GameStateRef`) self))
  (if _isinlight
    (`self.AffectHealth` (`self.DamageFromLight`)))
  (`KismetSystemLibrary.PrintString` (`KismetStringLibrary.Concat_StrStr` "Enemy Health: " (`KismetStringLibrary.Conv_DoubleToString` (`self.Health`))) true true (struct :`R` 1.0 :`G` 0.062269 :`B` 0.082164 :`A` 1.0)))

(event `self.AffectHealth`
  (params (Delta :type "Float (single-precision)"))
  (`self.CalculateHealth` Delta)
  (if (`self.isDead`)
    (`self.K2_DestroyActor`)))

(fn `UserConstructionScript`
  (`parent.UserConstructionScript`))