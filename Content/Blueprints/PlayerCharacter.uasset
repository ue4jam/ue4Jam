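; Player character with axis movement, a knockback melee attack, and health that drains outside of light.
; A looping timer checks the Light actors cached at BeginPlay by range and Visibility line trace, reduces health when none qualifies, and prints health.
; Basic attack impulses overlapping EnemyCharacters along control-rotation forward, scaled by Strength, then waits out a cooldown.
; Movement uses world axes and sets control rotation from axis input.
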(event `self.ReceiveBeginPlay`
  (`|ExecutionSequence`
    (:`then_0`
      (bind _outactors (`GameplayStatics.GetAllActorsOfClass` "/Script/Engine.Light"))
      (bind _output_get (set `self.LightSourceRefs` _outactors))
      (for _ _output_get
        _))
    (:`then_1`
      (`KismetSystemLibrary.K2_SetTimer` null "DamageIfNotInLight" 2.0 true))))

(event `self.ReceiveTick`
  (params (DeltaSeconds :type "Float (single-precision)")))

(event `DamageIfNotInLight`
  (`self.CalculateInLight`)
  (if (not (`self.inLight`))
    (`self.CalculateHealth` -1.0))
  (`KismetSystemLibrary.PrintString` (`KismetStringLibrary.Concat_StrStr` "Health: " (`KismetStringLibrary.Conv_DoubleToString` (`self.Health`)))))

(event `InputAxis|MoveUp`
  (params (AxisValue :type "Float (single-precision)"))
  ;[1 1 1] Movement/Rotation
  (`self.AddMovementInput` (1.0 0.0 0.0) AxisValue)
  (bind _returnvalue (`KismetMathLibrary.MakeVector` AxisValue (stale `InputAxis|MoveRight` AxisValue)))
  (if (> (`KismetMathLibrary.VSize` _returnvalue) 0.5) :!label _label
    (`Controller.SetControlRotation` (`self.GetController`) (`KismetMathLibrary.Conv_VectorToRotator` _returnvalue))))

(event `InputAxis|MoveRight`
  (params (AxisValue :type "Float (single-precision)"))
  ;[1 1 1] Movement/Rotation
  (`self.AddMovementInput` (0.0 1.0 0.0) AxisValue)
  (goto _label))

(event `InputAction|BasicAttack`
  (params (Key :type "Key Structure"))
  (bind _overlappingactors (`PrimitiveComponent.GetOverlappingActors` (`self.AttackArea`) "/Game/Blueprints/EnemyCharacter.EnemyCharacter_C"))
  ;[1 1 1] BasicAttack
  (:`Pressed`
    (if (`self.CanAttack`)
      (if (>= (`KismetArrayLibrary.Array_LastIndex` _overlappingactors) 0)
        (`self.SetCanAttack` false)
        (for _array_element _overlappingactors
          (bind _asenemy_character (cast `/Game/Blueprints/EnemyCharacter` _array_element))
          (bind _charactermovement (`Character.CharacterMovement` _asenemy_character))
          (`MovementComponent.StopMovementImmediately` _charactermovement)
          (`CharacterMovementComponent.AddImpulse` _charactermovement (`self.CalculateMeleeForce`) false))
        (`KismetSystemLibrary.Delay` (`self.AttackDelay`))
        (`self.SetCanAttack` true)))))

(fn `CalculateInLight`
  (for _array_element (`self.LightSourceRefs`)
    (if (< (`self.GetDistanceTo` self _array_element) 500.0)
      (bind (_outhit _returnvalue) (`KismetSystemLibrary.LineTraceSingle` (`self.K2_GetActorLocation` self) (`SceneComponent.K2_GetComponentLocation` (`Light.LightComponent` _array_element)) "TraceTypeQuery1"))
      (if (not _returnvalue)
        (set `self.inLight` true)
        (break)
        (else
          _)))
    (set `self.inLight` false))
  (return))

(fn `CalculateMeleeForce`
  (returns (MeleeForce :type "Vector Structure"))
  (return (* (`KismetMathLibrary.GetForwardVector` (`self.GetControlRotation`)) (`self.Strength`))))

(fn `SetAttackDelay`
  (params (AttackDelay :type "Float (double-precision)"))
  (set `self.AttackDelay` AttackDelay)
  (return))

(fn `SetCanAttack`
  (params (CanAttack :type Boolean))
  (set `self.CanAttack` CanAttack)
  (return))

(fn `UserConstructionScript`)