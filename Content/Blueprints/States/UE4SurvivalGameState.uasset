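; Game state for a survival game that tracks light sources and reports whether a given character is standing in light.
; It gathers actors tagged LightSource at BeginPlay, offers add and remove functions, and refreshes its character list on a looping timer.
; The light check prunes invalid sources, then looks for one within a fixed radius that has an unblocked visibility trace, ignoring all listed characters.
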(event `self.ReceiveBeginPlay`
  (`|ExecutionSequence`
    (:`then_0`
      (bind _outactors (`GameplayStatics.GetAllActorsWithTag` "LightSource"))
      (set `self.LightSourceRefs` _outactors))
    (:`then_1`
      (`KismetSystemLibrary.K2_SetTimer` null "GetCharacters" 5.0 true))))

(event `GetCharacters`
  (`self.GetAllCharacters`))

(fn `AddLightSource`
  (params (LightSource :type "Actor Object Reference"))
  (returns (Index :type Integer))
  (bind _returnvalue (`KismetArrayLibrary.Array_Add` (`self.LightSourceRefs`) LightSource))
  (return _returnvalue))

(fn `CheckIfInLight`
  (params (CharacterRef :type "/Game/Blueprints/Characters/BaseCharacterBP Object Reference"))
  (returns (IsInLight :type Boolean))
  (locals (BaseCharacterRef :type "/Game/Blueprints/Characters/BaseCharacterBP Object Reference") (InLight :type Boolean))
  (bind _basecharacterref (`local.BaseCharacterRef`))
  (set `local.BaseCharacterRef` CharacterRef)
  (`self.CheckValidLightSources`)
  (for _array_element (`self.GetLightSources`)
    (`/Engine/EditorBlueprintResources/StandardMacros.IsValid` _array_element
      (:`Is Valid`
        (if (<= (`self.GetDistanceTo` _basecharacterref _array_element) 500.0)
          (bind (_outhit _returnvalue) (`KismetSystemLibrary.LineTraceSingle` (`self.K2_GetActorLocation` _basecharacterref) (`self.K2_GetActorLocation` _array_element) "TraceTypeQuery1" false (`self.CharacterRefs`)))
          (if (not _returnvalue)
            (set `local.InLight` true)
            (break)
            (else
              _)))
        (set `local.InLight` false))))
  (return (`local.InLight`)))

(fn `CheckValidLightSources`
  (locals (IndeciesToRemove :type "Array of Integer"))
  (bind _indeciestoremove (`local.IndeciesToRemove`))
  (for (_array_element _array_index) (`self.LightSourceRefs`)
    (`/Engine/EditorBlueprintResources/StandardMacros.IsValid` _array_element
      (:`Is Not Valid`
        (`KismetArrayLibrary.Array_Add` (`local.IndeciesToRemove`) _array_index))))
  (if (>= (`KismetArrayLibrary.Array_LastIndex` _indeciestoremove) 0)
    (`self.RemoveLightSources` _indeciestoremove))
  (`KismetArrayLibrary.Array_Clear` _indeciestoremove)
  (return))

(fn `GetAllCharacters`
  (returns (Characters :type "Array of /Game/Blueprints/Characters/BaseCharacterBP Object Reference"))
  (bind _outactors (`GameplayStatics.GetAllActorsOfClass` "/Game/Blueprints/Characters/BaseCharacterBP.BaseCharacterBP_C"))
  (set `self.CharacterRefs` _outactors)
  (return _outactors))

(fn `GetLightSources`
  (returns (LightSourceRefs :type "Array of Actor Object Reference"))
  (return (`self.LightSourceRefs`)))

(fn `RemoveLightSources`
  (params (Index :type "Array of Integer"))
  (for _array_element Index
    (`KismetArrayLibrary.Array_Remove` (`self.LightSourceRefs`) _array_element)
    (return)))

(fn `UserConstructionScript`)