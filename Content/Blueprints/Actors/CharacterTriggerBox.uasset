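; CharacterTriggerBox is a trigger actor that shows a message and changes the player's health and light energy on overlap.
; Only actors that cast to PlayerCharacterBP are affected, and the character is sent DisplayMessage first.
; ResetHealth and ResetEnergy flags each choose between setting that stat to a fixed 100 or passing a configurable amount to AffectHealth or AffectLightEnergy.
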(event `self.ReceiveActorBeginOverlap`
  (params (OtherActor :type "Actor Object Reference"))
  (bind _asplayer_character_bp (cast `/Game/Blueprints/Characters/PlayerCharacterBP` OtherActor))
  (bind _output_get (set `self.Character` _asplayer_character_bp))
  (`/Game/Blueprints/Characters/PlayerCharacterBP.DisplayMessage` _output_get (`self.DisplayMessage`))
  (if (`self.ResetHealth`)
    (set `/Game/Blueprints/Characters/BaseCharacterBP.Health` 100.0 _output_get)
    (else
      (`/Game/Blueprints/Characters/PlayerCharacterBP.AffectHealth` _output_get (`self.AffectHealthAmount`))))
  (if (`self.ResetEnergy`)
    (set `/Game/Blueprints/Characters/PlayerCharacterBP.LightEnergy` 100.0 _output_get)
    (else
      (`/Game/Blueprints/Characters/PlayerCharacterBP.AffectLightEnergy` _output_get (`self.AffectEnergyAmount`)))))

(fn `UserConstructionScript`)