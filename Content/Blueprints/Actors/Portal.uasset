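; Portal is a destructible actor that spawns a LightKey at its transform when destroyed.
; The AffectHealth event adds a delta to Health through CalculateHealth, which then updates IsDead via CalculateIsDead.
; Once Health is zero or below, the actor destroys itself, and its Destroyed event spawns the key.
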(event `/Game/Blueprints/Interfaces/iDamageable.AffectHealth`
  (params (Delta :type "Float (single-precision)"))
  (`self.CalculateHealth` Delta)
  (if (`self.IsDead`)
    (`self.K2_DestroyActor`)))

(event `self.ReceiveDestroyed`
  (`|SpawnActorFromClass` "/Game/Blueprints/Actors/LightKey.LightKey_C" (`self.GetTransform` self) "Undefined" "OverrideRootScale" null null))

(fn `CalculateHealth`
  (params (Delta :type "Float (double-precision)"))
  (set `self.Health` (+ (`self.Health`) Delta))
  (`self.CalculateIsDead`)
  (return))

(fn `CalculateIsDead`
  (set `self.IsDead` (<= (`self.Health`) 0.0))
  (return))

(fn `UserConstructionScript`)