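; Projectile actor that damages non-friendly actors on contact and then destroys itself.
; On overlap, it sends Damage through the IDamageable interface's AffectHealthMessage, skipping damageable actors tagged "Friendly" without being destroyed.
; Overlapping any non-damageable actor destroys it regardless of tag.
; A blocking hit destroys it without applying damage, unless the other actor is tagged "Friendly".
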(event `self.ReceiveActorBeginOverlap`
  (params (OtherActor :type "Actor Object Reference"))
  (if (`KismetSystemLibrary.DoesImplementInterface` OtherActor "/Game/Blueprints/Interfaces/iDamageable.iDamageable_C")
    (if (not (`self.ActorHasTag` OtherActor "Friendly"))
      (message `/Game/Blueprints/Interfaces/iDamageable.AffectHealth` OtherActor (`self.Damage`))
      (`self.K2_DestroyActor` :!label _label))
    (else
      (goto _label))))

(event `self.ReceiveHit`
  (params (MyComp :type "PrimitiveComponent Object Reference") (Other :type "Actor Object Reference") (OtherComp :type "PrimitiveComponent Object Reference") (bSelfMoved :type Boolean) (HitLocation :type "Vector Structure") (HitNormal :type "Vector Structure") (NormalImpulse :type "Vector Structure") (Hit :type "HitResult Structure (by ref)"))
  (if (not (`self.ActorHasTag` Other "Friendly"))
    (`self.K2_DestroyActor`)))

(fn `UserConstructionScript`)