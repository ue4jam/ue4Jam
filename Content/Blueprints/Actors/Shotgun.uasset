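; Shotgun weapon actor that fires a burst of five ShotgunProjectile actors at once.
; The SpawnProjectile event calls SpawnShotgunProjectile, which spawns one projectile at each of five spawn point components, so their fixed transforms define the pellet pattern.
; An unconnected loop that spawns projectiles with randomised location and roll offsets remains in the graph and never runs.
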(event `self.SpawnProjectile`
  (`self.SpawnShotgunProjectile`))

(fn `SpawnShotgunProjectile`
  (locals (Count :type Integer))
  (`|SpawnActorFromClass` "/Game/Blueprints/Actors/ShotgunProjectile.ShotgunProjectile_C" (`SceneComponent.K2_GetComponentToWorld` (`self.ProjectileSpawnPoint`)) "Undefined" "OverrideRootScale" null null)
  (`|SpawnActorFromClass` "/Game/Blueprints/Actors/ShotgunProjectile.ShotgunProjectile_C" (`SceneComponent.K2_GetComponentToWorld` (`self.ProjectileSpawnPoint2`)) "Undefined" "OverrideRootScale" null null)
  (`|SpawnActorFromClass` "/Game/Blueprints/Actors/ShotgunProjectile.ShotgunProjectile_C" (`SceneComponent.K2_GetComponentToWorld` (`self.ProjectileSpawnPoint3`)) "Undefined" "OverrideRootScale" null null)
  (`|SpawnActorFromClass` "/Game/Blueprints/Actors/ShotgunProjectile.ShotgunProjectile_C" (`SceneComponent.K2_GetComponentToWorld` (`self.ProjectileSpawnPoint4`)) "Undefined" "OverrideRootScale" null null)
  (`|SpawnActorFromClass` "/Game/Blueprints/Actors/ShotgunProjectile.ShotgunProjectile_C" (`SceneComponent.K2_GetComponentToWorld` (`self.ProjectileSpawnPoint5`)) "Undefined" "OverrideRootScale" null null))

(fn `UserConstructionScript`
  (`parent.UserConstructionScript`))