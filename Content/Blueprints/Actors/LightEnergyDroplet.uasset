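; LightEnergyDroplet is a pickup actor that passes a small amount of light energy to friendly actors that touch it.
; The construction script rolls a small random whole-number Energy value for each droplet.
; On overlap, it checks that the other actor implements the ILightEnergy interface and carries the Friendly tag, then sends Energy through the AffectLightEnergy interface message and destroys itself.
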(event `self.ReceiveActorBeginOverlap`
  (params (OtherActor :type "Actor Object Reference"))
  (if (`KismetSystemLibrary.DoesImplementInterface` OtherActor "/Game/Blueprints/Interfaces/iLightEnergy.iLightEnergy_C")
    (if (`self.ActorHasTag` OtherActor "Friendly")
      (message `/Game/Blueprints/Interfaces/iLightEnergy.AffectLightEnergy` OtherActor (`self.Energy`))
      (`self.K2_DestroyActor`))))

(fn `UserConstructionScript`
  (set `self.Energy` (`KismetMathLibrary.Conv_IntToDouble` (`KismetMathLibrary.RandomIntegerInRange` 1 3))))